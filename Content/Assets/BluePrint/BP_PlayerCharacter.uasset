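; Player character Blueprint that supplies timeline-driven forward movement for animations and dodges.
; MoveDuringAnim and DodgeMoving lerp the actor forward by GetAnimMoveSpeed and DodgeVal respectively, using swept location updates with timeline tracks as alpha.
; Buffer runs an unswept forward lerp by BufferAmount until StopBuffer halts it, but its alpha is fixed at zero, so it produces no displacement.
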(event EventBeginPlay)

(event Collision|EventActorBeginOverlap
  (params (OtherActor :type Actor%20Object%20Reference)))

(event EventTick
  (params (DeltaSeconds :type Float%20%28single-precision%29)))

(event EventBuffer
  (params (BufferAmount :type Float%20%28single-precision%29))
  (bind _returnvalue (Transformation|GetActorLocation))
  ;[1 1 1] Buffer
  (Timeline|Buffer%20Timeline PlayFromStart
    (:Update
      (Transformation|SetActorLocation (Math|Vector|Lerp(Vector) _returnvalue (+ (* (Transformation|GetActorForwardVector) BufferAmount) _returnvalue) 0.0) false false))))

(event EventStopBuffer
  (bind _returnvalue (Transformation|GetActorLocation))
  ;[1 1 1] Buffer
  (Timeline|Buffer%20Timeline Stop
    (:Update
      (Transformation|SetActorLocation (Math|Vector|Lerp(Vector) _returnvalue (+ (* (Transformation|GetActorForwardVector) (stale EventBuffer BufferAmount)) _returnvalue) 0.0) false false))))

(event EventMoveDuringAnim
  (bind _returnvalue (Transformation|GetActorLocation))
  (bind _returnvalue_2 (Class|DYCharacter|GetAnimMoveSpeed))
  (bind _newtrack_0 (Timeline|Timeline PlayFromStart)
    (:Update
      (Transformation|SetActorLocation (Math|Vector|Lerp(Vector) _returnvalue (+ (* (Transformation|GetActorForwardVector) _returnvalue_2) _returnvalue) _newtrack_0) true false))))

(event EventDodgeMoving
  (bind _returnvalue (Transformation|GetActorLocation))
  ;[1 1 1] DodgeMove
  (bind _newtrack_0 (Timeline|DodgeMove PlayFromStart)
    (:Update
      (Transformation|SetActorLocation (Math|Vector|Lerp(Vector) _returnvalue (+ _returnvalue (* (Transformation|GetActorForwardVector) (Variables|Default|GetDodgeVal))) _newtrack_0) true false))))

(fn ConstructionScript)